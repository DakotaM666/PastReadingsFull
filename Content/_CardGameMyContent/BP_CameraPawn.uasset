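; Camera pawn for the card game that enables mouse interaction and provides keyboard shortcuts for the deck.
; On BeginPlay it turns on click and mouse-over events for player controller 0.
; K and B find the "DeckControl"-tagged actor nearest the world origin and send it interface messages: K to draw cards, B to show hand cards as a dev function.
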(event `Key|K`
  (params (Key :type "Key Structure"))
  (:`Pressed`
    (bind _outactors (`GameplayStatics.GetAllActorsWithTag` "DeckControl"))
    (message `/Game/_CardGameMyContent/BPI_BrainCardGame.DrawCards` (`.ReturnValue` (`GameplayStatics.FindNearestActor` (0.0 0.0 0.0) _outactors)))))

(event `self.ReceiveBeginPlay`
  (bind _returnvalue (`GameplayStatics.GetPlayerController` 0))
  (set `PlayerController.bEnableClickEvents` true _returnvalue)
  (set `PlayerController.bEnableMouseOverEvents` true _returnvalue))

(event `Key|B`
  (params (Key :type "Key Structure"))
  (:`Pressed`
    (bind _outactors (`GameplayStatics.GetAllActorsWithTag` "DeckControl"))
    (message `/Game/_CardGameMyContent/BPI_BrainCardGame.DEV_ShowHandCards` (`.ReturnValue` (`GameplayStatics.FindNearestActor` (0.0 0.0 0.0) _outactors)))))

(fn `UserConstructionScript`)