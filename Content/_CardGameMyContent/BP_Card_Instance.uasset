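; A single card actor in a card game: it animates placement, shuffle, flip, defeat and game-end poses according to its CardZone.
; Cursor events, mostly gated by the Deck's CanInteract, drive hover, moves between hand and play, and swap handling.
; It reports clicks, moves and sounds to tag-found DeckControl actors via messages.
; The construction script sets the face texture on dynamic materials, whose MovementHover parameter Tick interpolates for hover.
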(event `self.ReceiveBeginPlay`
  (bind _sm_cardtemplate (`self.SM_CardTemplate`))
  (bind _sm_cardtemplate_2 (`self.SM_CardTemplate`))
  (bind _sm_cardtemplate_3 (`self.SM_CardTemplate`))
  (bind _sm_cardtemplate_4 (`self.SM_CardTemplate`))
  (bind _sm_cardtemplate_5 (`self.SM_CardTemplate`))
  (`KismetSystemLibrary.MoveComponentTo` _sm_cardtemplate_5 (`KismetMathLibrary.MakeVector` (* (`self.RelativeXPos`) -50.0)) (struct :`Pitch` 180.0 :`Yaw` 180.0 :`Roll` -90.0) true true 0.0 true)
  (set `self.ShuffleCount` (`KismetMathLibrary.Conv_BoolToInt` (and (== (`self.CardZone`) 0) (== (`self.RelativeXPos`) 1))))
  (if (or (== (`self.CardZone`) 1) (== (`self.CardZone`) 4))
    (`KismetSystemLibrary.MoveComponentTo` _sm_cardtemplate_5 (`KismetMathLibrary.MakeVector` (* (`self.RelativeXPos`) -50.0)) (struct :`Yaw` 180.0 :`Roll` -90.0) true true 0.5 true :!label _label)
    (elif (`KismetMathLibrary.Conv_IntToBool` (`self.ShuffleCount`))
      (bind _output_get (set `self.RelativeXPos` 0))
      (`KismetSystemLibrary.MoveComponentTo` _sm_cardtemplate_5 (`KismetMathLibrary.MakeVector` (* _output_get -50.0)) (struct :`Pitch` 180.0 :`Yaw` 180.0 :`Roll` -90.0) true true 0.2 true)
      (bind _output_get_2 (set `self.RelativeXPos` 1))
      (`KismetSystemLibrary.MoveComponentTo` _sm_cardtemplate_2 (`KismetMathLibrary.MakeVector` (* _output_get_2 -50.0)) (struct :`Pitch` 180.0 :`Yaw` 180.0 :`Roll` -90.0) true true 0.2 true)
      (bind _output_get_3 (set `self.RelativeXPos` 0))
      (`KismetSystemLibrary.MoveComponentTo` _sm_cardtemplate_2 (`KismetMathLibrary.MakeVector` (* _output_get_3 -50.0)) (struct :`Pitch` 180.0 :`Yaw` 180.0 :`Roll` -90.0) true true 0.2 true)
      (bind _output_get_4 (set `self.RelativeXPos` 1))
      (`KismetSystemLibrary.MoveComponentTo` _sm_cardtemplate_3 (`KismetMathLibrary.MakeVector` (* _output_get_4 -50.0)) (struct :`Pitch` 180.0 :`Yaw` 180.0 :`Roll` -90.0) true true 0.2 true)
      (bind _output_get_5 (set `self.RelativeXPos` 0))
      (`KismetSystemLibrary.MoveComponentTo` _sm_cardtemplate_3 (`KismetMathLibrary.MakeVector` (* _output_get_5 -50.0)) (struct :`Pitch` 180.0 :`Yaw` 180.0 :`Roll` -90.0) true true 0.2 true)
      (bind _output_get_6 (set `self.RelativeXPos` 1))
      (`KismetSystemLibrary.MoveComponentTo` _sm_cardtemplate_4 (`KismetMathLibrary.MakeVector` (* _output_get_6 -50.0)) (struct :`Pitch` 180.0 :`Yaw` 180.0 :`Roll` -90.0) true true 0.2 true)
      (bind _output_get_7 (set `self.RelativeXPos` 0))
      (`KismetSystemLibrary.MoveComponentTo` _sm_cardtemplate_4 (`KismetMathLibrary.MakeVector` (* _output_get_7 -50.0)) (struct :`Pitch` 180.0 :`Yaw` 180.0 :`Roll` -90.0) true true 0.2 true)
      (bind _output_get_8 (set `self.RelativeXPos` 1))
      (`KismetSystemLibrary.MoveComponentTo` _sm_cardtemplate (`KismetMathLibrary.MakeVector` (* _output_get_8 -50.0)) (struct :`Pitch` 180.0 :`Yaw` 180.0 :`Roll` -90.0) true true 0.2 true)
      (bind _output_get_9 (set `self.RelativeXPos` 0))
      (`KismetSystemLibrary.MoveComponentTo` _sm_cardtemplate (`KismetMathLibrary.MakeVector` (* _output_get_9 -50.0)) (struct :`Pitch` 180.0 :`Yaw` 180.0 :`Roll` -90.0) true true 0.2 true)
      (elif (== (`self.CardZone`) 3)
        (`KismetSystemLibrary.MoveComponentTo` (`self.SM_CardTemplate`) (`KismetMathLibrary.MakeVector` (* (`self.RelativeXPos`) -50.0) 50.0) (struct :`Yaw` 180.0 :`Roll` -90.0) true true 0.0 true)
        (`KismetSystemLibrary.Delay` (/ (`self.EnemyCardNumber`) 5.0))
        (`KismetSystemLibrary.MoveComponentTo` (`self.SM_CardTemplate`) (`KismetMathLibrary.MakeVector` (* (`self.RelativeXPos`) -50.0)) (struct :`Yaw` 180.0 :`Roll` -90.0) true true 1.0 true)))))

(event `/Game/_CardGameMyContent/BPI_BrainCardGame.RefreshPosCard`
  (goto _label))

(event `self.ReceiveTick`
  (params (DeltaSeconds :type "Float (single-precision)"))
  (bind _returnvalue (`self.K2_GetActorLocation`))
  (bind _cardzone (`self.CardZone`))
  (switch `int` (`self.CardZone`)
    (:`0`
      (`self.K2_SetActorRotation` (struct)))
    (:`1`
      (`self.K2_SetActorLocation` (`KismetMathLibrary.VInterpTo` _returnvalue (`KismetMathLibrary.MakeVector` (.x _returnvalue) (.y _returnvalue) 120.0) DeltaSeconds 5.0) :!label _label_2)
      (if (`self.BeingHovered`)
        (switch `int` _cardzone
          (:`1`
            (`self.HoverMovement` 20.0 DeltaSeconds))
          (:`2`
            (`self.HoverMovement` -20.0 DeltaSeconds :!label _label_3))
          (:`4`
            (goto _label_3)))
        (else
          (switch `int` _cardzone
            (:`1`
              (`self.HoverMovement` 0.0 DeltaSeconds))
            (:`2`
              (`self.HoverMovement` 0.0 DeltaSeconds :!label _label_4))
            (:`4`
              (goto _label_4))))))
    (:`2`
      (goto _label_2))
    (:`4`
      (goto _label_2))))

(event `/Game/_CardGameMyContent/BPI_BrainCardGame.FlipCard`
  (`KismetSystemLibrary.PrintString` "Flipping Card")
  (`KismetSystemLibrary.MoveComponentTo` (`self.SM_CardTemplate`) (`KismetMathLibrary.MakeVector` (* (`self.RelativeXPos`) -50.0)) (struct :`Pitch` 180.0 :`Yaw` 180.0 :`Roll` -90.0) true true 0.5 true))

(event `self.ReceiveActorBeginCursorOver`
  (bind _cardzone (`self.CardZone`))
  (bind _returnvalue (== _cardzone 4))
  (bind _returnvalue_2 (`GameplayStatics.GetActorOfClass` "/Game/_CardGameMyContent/Deck.Deck_C"))
  (if (`/Game/_CardGameMyContent/Deck.CanInteract` _returnvalue_2)
    (if (or (== _cardzone 1) (== _cardzone 2) _returnvalue)
      (set `self.BeingHovered` true)
      (bind _outactors (`GameplayStatics.GetAllActorsWithTag` "DeckControl"))
      (message `/Game/_CardGameMyContent/BPI_BrainCardGame.SlideCardSoundCall` (`.ReturnValue` (`GameplayStatics.FindNearestActor` (0.0 0.0 0.0) _outactors)) 1)
      (if _returnvalue
        (bind _outactors_2 (`GameplayStatics.GetAllActorsWithTag` "FloatingMessage"))
        (message `/Game/_CardGameMyContent/BPI_BrainCardGame.SetFace` (`.ReturnValue` (`GameplayStatics.FindNearestActor` (0.0 0.0 0.0) _outactors_2)) "/Game/_CardGameMyContent/_UI/ConfirmTextPanelHighlight.ConfirmTextPanelHighlight" false)))))

(event `/Game/_CardGameMyContent/BPI_BrainCardGame.DefeatedCard`
  (if (== (`self.CardZone`) 2)
    (`KismetSystemLibrary.MoveComponentTo` (`self.SM_CardTemplate`) (`KismetMathLibrary.MakeVector` (* (`self.RelativeXPos`) -50.0) (* (`KismetMathLibrary.Conv_IntToDouble` (`self.RelativeYPos`)) 50.0) -10.0) (struct :`Yaw` 210.0 :`Roll` -90.0) false true 0.2 true)
    (bind _outactors (`GameplayStatics.GetAllActorsWithTag` "DeckControl"))
    (message `/Game/_CardGameMyContent/BPI_BrainCardGame.SlideCardSoundCall` (`.ReturnValue` (`GameplayStatics.FindNearestActor` (0.0 0.0 0.0) _outactors)) 0)
    (else
      (`KismetSystemLibrary.MoveComponentTo` (`self.SM_CardTemplate`) (`KismetMathLibrary.MakeVector` (* (`self.RelativeXPos`) -50.0) 0.0 10.0) (struct :`Pitch` 180.0 :`Yaw` 210.0 :`Roll` -90.0) false true 0.2 true)
      (bind _outactors_2 (`GameplayStatics.GetAllActorsWithTag` "DeckControl"))
      (message `/Game/_CardGameMyContent/BPI_BrainCardGame.SlideCardSoundCall` (`.ReturnValue` (`GameplayStatics.FindNearestActor` (0.0 0.0 0.0) _outactors_2)) 0))))

(event `self.ReceiveActorEndCursorOver`
  (bind _cardzone (`self.CardZone`))
  (bind _returnvalue (== _cardzone 4))
  (if (or (== _cardzone 1) (== _cardzone 2) _returnvalue)
    (set `self.BeingHovered` false)
    (set `self.WasClicked` false)
    (if _returnvalue
      (bind _outactors (`GameplayStatics.GetAllActorsWithTag` "FloatingMessage"))
      (message `/Game/_CardGameMyContent/BPI_BrainCardGame.SetFace` (`.ReturnValue` (`GameplayStatics.FindNearestActor` (0.0 0.0 0.0) _outactors)) "/Game/_CardGameMyContent/_UI/ConfirmTextPanel.ConfirmTextPanel" false))))

(event `self.ReceiveActorOnClicked`
  (params (ButtonPressed :type "Key Structure"))
  (bind _returnvalue (`GameplayStatics.GetActorOfClass` "/Game/_CardGameMyContent/Deck.Deck_C"))
  (if (`/Game/_CardGameMyContent/Deck.CanInteract` _returnvalue)
    (set `self.WasClicked` true)
    (bind _outactors (`GameplayStatics.GetAllActorsWithTag` "DeckControl"))
    (message `/Game/_CardGameMyContent/BPI_BrainCardGame.ClickedCard` (`.ReturnValue` (`GameplayStatics.FindNearestActor` (0.0 0.0 0.0) _outactors)) (make `/Game/_CardGameMyContent/STRUCT_Card` (`KismetSystemLibrary.GetDisplayName` (`self.Cara`)) self) (`self.CardZone`) (`self.RelativeXPos`))
    (bind _outactors_2 (`GameplayStatics.GetAllActorsWithTag` "DeckControl"))
    (message `/Game/_CardGameMyContent/BPI_BrainCardGame.SlideCardSoundCall` (`.ReturnValue` (`GameplayStatics.FindNearestActor` (0.0 0.0 0.0) _outactors_2)) 0)))

(event `self.ReceiveActorOnReleased`
  (params (ButtonReleased :type "Key Structure"))
  (bind _cardzone (`self.CardZone`))
  (bind _returnvalue (`GameplayStatics.GetActorOfClass` "/Game/_CardGameMyContent/Deck.Deck_C"))
  (if (`/Game/_CardGameMyContent/Deck.CanInteract` _returnvalue)
    (if (`self.WasClicked`)
      (if (== (`self.CardZone`) 1)
        (bind _output_get (set `self.RelativeYPos` 1))
        (`KismetSystemLibrary.MoveComponentTo` (`self.SM_CardTemplate`) (`KismetMathLibrary.MakeVector` (* (`self.RelativeXPos`) -50.0) (* (`KismetMathLibrary.Conv_IntToDouble` _output_get) 50.0)) (struct :`Yaw` 180.0 :`Roll` -90.0) true true 0.1 true)
        (set `self.CardZone` 2)
        (set `self.BeingHovered` false)
        (bind _outactors (`GameplayStatics.GetAllActorsWithTag` "DeckControl"))
        (message `/Game/_CardGameMyContent/BPI_BrainCardGame.CardToPlay` (`.ReturnValue` (`GameplayStatics.FindNearestActor` (0.0 0.0 0.0) _outactors)) (make `/Game/_CardGameMyContent/STRUCT_Card` (`KismetSystemLibrary.GetDisplayName` (`self.Cara`)) self))
        (elif (== _cardzone 2)
          (bind _output_get_2 (set `self.RelativeYPos` 0))
          (`KismetSystemLibrary.MoveComponentTo` (`self.SM_CardTemplate`) (`KismetMathLibrary.MakeVector` (* (`self.RelativeXPos`) -50.0) (* (`KismetMathLibrary.Conv_IntToDouble` _output_get_2) 50.0)) (struct :`Yaw` 180.0 :`Roll` -90.0) true true 0.1 true)
          (set `self.CardZone` 1)
          (set `self.BeingHovered` false)
          (bind _outactors_2 (`GameplayStatics.GetAllActorsWithTag` "DeckControl"))
          (message `/Game/_CardGameMyContent/BPI_BrainCardGame.CardToHand` (`.ReturnValue` (`GameplayStatics.FindNearestActor` (0.0 0.0 0.0) _outactors_2)) (make `/Game/_CardGameMyContent/STRUCT_Card` (`KismetSystemLibrary.GetDisplayName` (`self.Cara`)) self))))
      (else
        (bind _outactors_3 (`GameplayStatics.GetAllActorsWithTag` "DeckControl"))
        (message `/Game/_CardGameMyContent/BPI_BrainCardGame.ReleasedCard` (`.ReturnValue` (`GameplayStatics.FindNearestActor` (0.0 0.0 0.0) _outactors_3)) (make `/Game/_CardGameMyContent/STRUCT_Card` (`KismetSystemLibrary.GetDisplayName` (`self.Cara`)) self) _cardzone (`self.RelativeXPos`))))))

(event `/Game/_CardGameMyContent/BPI_BrainCardGame.SwitchPlacesReleased`
  (params (ClickedPos :type Integer) (ReleasedPos :type Integer))
  (bind _returnvalue (`KismetMathLibrary.MakeVector` (* (`self.RelativeXPos`) -50.0) (* (`self.RelativeYPos`) 50.0)))
  (bind _returnvalue_2 (`GameplayStatics.GetActorOfClass` "/Game/_CardGameMyContent/Deck.Deck_C"))
  (set `/Game/_CardGameMyContent/Deck.CanInteract` false _returnvalue_2)
  (set `self.RelativeXPos` ClickedPos)
  (switch `int` (`self.CardZone`)
    (:`1`
      (bind _outactors (`GameplayStatics.GetAllActorsWithTag` "DeckControl" :!label _label_5))
      (message `/Game/_CardGameMyContent/BPI_BrainCardGame.SlideCardSoundCall` (`.ReturnValue` (`GameplayStatics.FindNearestActor` (0.0 0.0 0.0) _outactors)) 3))
    (:`2`
      (bind _outactors_2 (`GameplayStatics.GetAllActorsWithTag` "DeckControl" :!label _label_6))
      (message `/Game/_CardGameMyContent/BPI_BrainCardGame.SlideCardSoundCall` (`.ReturnValue` (`GameplayStatics.FindNearestActor` (0.0 0.0 0.0) _outactors_2)) 3)))
  (`KismetSystemLibrary.MoveComponentTo` (`self.SM_CardTemplate`) _returnvalue (struct :`Yaw` 180.0 :`Roll` -90.0) true true 0.3 true)
  (`KismetSystemLibrary.PrintString` (`KismetStringLibrary.BuildString_Vector` "MovedHAND - " "" _returnvalue))
  (bind _returnvalue_3 (`GameplayStatics.GetActorOfClass` "/Game/_CardGameMyContent/Deck.Deck_C"))
  (set `/Game/_CardGameMyContent/Deck.CanInteract` true _returnvalue_3))

(event `/Game/_CardGameMyContent/BPI_BrainCardGame.SwitchPlacesClicked`
  (params (ClickedPos :type Integer) (ReleasedPos :type Integer))
  (bind _returnvalue (`GameplayStatics.GetActorOfClass` "/Game/_CardGameMyContent/Deck.Deck_C"))
  (set `/Game/_CardGameMyContent/Deck.CanInteract` false _returnvalue)
  (set `self.RelativeXPos` ReleasedPos)
  (switch `int` (`self.CardZone`)
    (:`1`
      (goto _label_5))
    (:`2`
      (goto _label_6))))

(event `/Game/_CardGameMyContent/BPI_BrainCardGame.WonGame`
  (`KismetSystemLibrary.MoveComponentTo` (`self.SM_CardTemplate`) (`KismetMathLibrary.MakeVector` 80.0 -50.0 15.0) (struct :`Yaw` 180.0 :`Roll` -45.0) true true 0.5 true))

(event `/Game/_CardGameMyContent/BPI_BrainCardGame.LostGame`
  (`KismetSystemLibrary.MoveComponentTo` (`self.SM_CardTemplate`) (`KismetMathLibrary.MakeVector` 80.0 -50.0 15.0) (struct :`Roll` -135.0) true true 0.5 true))

(fn `HoverMovement`
  (params (Target :type "Float (double-precision)" :default 20.0) (DeltaTime :type "Float (double-precision)"))
  (if (not (== (`self.RiseMovement`) Target))
    (bind _output_get (set `self.RiseMovement` (`KismetMathLibrary.FInterpTo` (`KismetMathLibrary.FInterpTo` (`self.RiseMovement`) Target DeltaTime 10.0) Target DeltaTime 10.0)))
    (`MeshComponent.SetScalarParameterValueOnMaterials` (`self.SM_CardTemplate`) "MovementHover" _output_get)))

(fn `UserConstructionScript`
  (bind _returnvalue (`PrimitiveComponent.CreateDynamicMaterialInstance` (`self.SM_CardTemplate`) 0 "/Game/_CardGameMyContent/M_Front_Inst.M_Front_Inst" "None"))
  (`MaterialInstanceDynamic.SetTextureParameterValue` _returnvalue "Cara" (`self.Cara`))
  (`MaterialInstanceDynamic.SetScalarParameterValue` _returnvalue "MovementHover" 0.0)
  (bind _returnvalue_2 (`PrimitiveComponent.CreateDynamicMaterialInstance` (`self.SM_CardTemplate`) 1 "/Game/_CardGameMyContent/M_Back_Inst.M_Back_Inst" "None"))
  (`MaterialInstanceDynamic.SetScalarParameterValue` _returnvalue_2 "MovementHover" 0.0))