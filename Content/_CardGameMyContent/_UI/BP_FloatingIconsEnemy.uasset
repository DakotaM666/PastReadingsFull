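; BP_FloatingIconsEnemy is a card game actor that shows a card icon on a plane and can be marked as enemy or player score.
; Its construction script creates a dynamic material on the plane with the initial Cara texture and a white color filter.
; SetFace swaps the icon texture at runtime.
; The two tag events tint it red or cyan and replace all actor tags with EnemyScore or PlayerScore.
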(event `/Game/_CardGameMyContent/BPI_BrainCardGame.SetFace`
  (params (Cara :type "Texture Object Reference") (Force :type Boolean))
  (`MaterialInstanceDynamic.SetTextureParameterValue` (`self.DynamicMaterial`) "CardIcon" Cara))

(event `/Game/_CardGameMyContent/BPI_BrainCardGame.MakeEnemyTagScore`
  (bind _tags (`self.Tags`))
  (`MaterialInstanceDynamic.SetVectorParameterValue` (`self.DynamicMaterial`) "ColorFilter" (`KismetMathLibrary.MakeColor` 1.0 0.2 0.2))
  (`KismetArrayLibrary.Array_Clear` _tags)
  (`KismetArrayLibrary.Array_Add` _tags "EnemyScore"))

(event `/Game/_CardGameMyContent/BPI_BrainCardGame.MakePlayerTagScore`
  (bind _tags (`self.Tags`))
  (`MaterialInstanceDynamic.SetVectorParameterValue` (`self.DynamicMaterial`) "ColorFilter" (`KismetMathLibrary.MakeColor` 0.2 1.0 1.0))
  (`KismetArrayLibrary.Array_Clear` _tags)
  (`KismetArrayLibrary.Array_Add` _tags "PlayerScore"))

(fn `UserConstructionScript`
  (bind _returnvalue (`PrimitiveComponent.CreateDynamicMaterialInstance` (`self.Plane`) 0 "/Game/_CardGameMyContent/_UI/FloatingIconsMaterialInstance.FloatingIconsMaterialInstance" "None"))
  (bind _output_get (set `self.DynamicMaterial` _returnvalue))
  (`MaterialInstanceDynamic.SetTextureParameterValue` _output_get "CardIcon" (`self.Cara`))
  (`MaterialInstanceDynamic.SetVectorParameterValue` _output_get "ColorFilter" (`KismetMathLibrary.MakeColor` 1.0 1.0 1.0)))