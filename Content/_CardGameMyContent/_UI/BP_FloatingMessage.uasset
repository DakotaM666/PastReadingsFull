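; BP_FloatingMessage shows a card face icon on a plane in the card game, dimmed or fully opaque.
; The construction script creates a dynamic material instance on the plane, applies the face texture and starts at half opacity.
; UpdateFloatingMessageOpacity switches to full opacity when the play has three elements.
; SetFace changes the texture only when forced or when the Opacity flag is set.
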(event `/Game/_CardGameMyContent/BPI_BrainCardGame.SetFace`
  (params (Cara :type "Texture Object Reference") (Force :type Boolean))
  (if (or Force (`self.Opacity`))
    (bind _output_get (set `self.Cara` Cara))
    (`MaterialInstanceDynamic.SetTextureParameterValue` (`self.DynamicMaterial`) "CardIcon" _output_get)))

(event `/Game/_CardGameMyContent/BPI_BrainCardGame.UpdateFloatingMessageOpacity`
  (params (DoesPlayHave3Elements :type Boolean))
  (bind _dynamicmaterial (`self.DynamicMaterial`))
  (bind _output_get (set `self.Opacity` DoesPlayHave3Elements))
  (if _output_get
    (`MaterialInstanceDynamic.SetScalarParameterValue` _dynamicmaterial "Opacity" 1.0)
    (else
      (`MaterialInstanceDynamic.SetScalarParameterValue` _dynamicmaterial "Opacity" 0.5))))

(fn `UserConstructionScript`
  (bind _returnvalue (`PrimitiveComponent.CreateDynamicMaterialInstance` (`self.Plane`) 0 "/Game/_CardGameMyContent/_UI/FloatingIconsMaterialInstance.FloatingIconsMaterialInstance" "None"))
  (bind _output_get (set `self.DynamicMaterial` _returnvalue))
  (`MaterialInstanceDynamic.SetTextureParameterValue` _output_get "CardIcon" (`self.Cara`))
  (`MaterialInstanceDynamic.SetScalarParameterValue` _returnvalue "Opacity" 0.5))