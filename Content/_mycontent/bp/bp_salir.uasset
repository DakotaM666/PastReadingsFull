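; Exit interactable that takes the player out of the house by loading the garden level.
; A sphere trigger shows a prompt widget on overlap and hides it on end overlap, without filtering which actor overlaps.
; The Interact event opens Lvl_garden only while the player pawn overlaps the box component.
; CheckSpeaking always returns false.
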(event `self.Sphere.OnComponentBeginOverlap`
  (params (OverlappedComponent :type "PrimitiveComponent Object Reference") (OtherActor :type "Actor Object Reference") (OtherComp :type "PrimitiveComponent Object Reference") (OtherBodyIndex :type Integer) (bFromSweep :type Boolean) (SweepResult :type "HitResult Structure (by ref)"))
  ;[0.531 0.4268 1] visibilidad widget por cercania
  (`SceneComponent.SetHiddenInGame` (`self.Widget`) false false))

(event `self.Sphere.OnComponentEndOverlap`
  (params (OverlappedComponent :type "PrimitiveComponent Object Reference") (OtherActor :type "Actor Object Reference") (OtherComp :type "PrimitiveComponent Object Reference") (OtherBodyIndex :type Integer))
  ;[0.531 0.4268 1] visibilidad widget por cercania
  (`SceneComponent.SetHiddenInGame` (`self.Widget`) true false))

(event `/Game/ThirdPerson/Blueprints/bpi_player.Interact`
  ;[1 0.4943 0.7672] salir casa
  (if (`PrimitiveComponent.IsOverlappingActor` (`self.Box`) (`GameplayStatics.GetPlayerPawn` 0))
    (`GameplayStatics.OpenLevelBySoftObjectPtr` "/Game/_mycontent/levels/lvl_garden.lvl_garden")))

(fn `CheckSpeaking`
  (returns (bSpeak :type Boolean))
  (return false))

(fn `UserConstructionScript`)