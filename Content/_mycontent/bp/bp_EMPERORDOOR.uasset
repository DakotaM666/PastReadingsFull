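; Emperor door interactable that awards card 4 and shows its prompt widget while something overlaps its proximity sphere.
; On Interact, if the player is inside the box and lacks the card, it saves their location, rotation and whether the level is the garden to the GameInstance.
; It then plays a sound, records the found card, plays a cinematic and opens the card tabletop level after fixed delays.
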(event `self.Sphere.OnComponentBeginOverlap`
  (params (OverlappedComponent :type "PrimitiveComponent Object Reference") (OtherActor :type "Actor Object Reference") (OtherComp :type "PrimitiveComponent Object Reference") (OtherBodyIndex :type Integer) (bFromSweep :type Boolean) (SweepResult :type "HitResult Structure (by ref)"))
  ;[0.531 0.4268 1] visibilidad widget por cercania
  (`SceneComponent.SetHiddenInGame` (`self.Widget`) false false))

(event `self.Sphere.OnComponentEndOverlap`
  (params (OverlappedComponent :type "PrimitiveComponent Object Reference") (OtherActor :type "Actor Object Reference") (OtherComp :type "PrimitiveComponent Object Reference") (OtherBodyIndex :type Integer))
  ;[0.531 0.4268 1] visibilidad widget por cercania
  (`SceneComponent.SetHiddenInGame` (`self.Widget`) true false))

(event `self.Interact`
  (bind _returnvalue (`GameplayStatics.GetPlayerPawn` 0))
  ;[1 0.4943 0.7672] salir casa
  (if (`PrimitiveComponent.IsOverlappingActor` (`self.Box`) (`GameplayStatics.GetPlayerPawn` 0))
    (bind _asbp_past_readings_game_instance (cast `/Game/_mycontent/bp/bp_PastReadingsGameInstance` (`GameplayStatics.GetGameInstance`)))
    (if (not (`KismetArrayLibrary.Array_Contains` (`/Game/_mycontent/bp/bp_PastReadingsGameInstance.CardsGot` _asbp_past_readings_game_instance) 4))
      (set `/Game/_mycontent/bp/bp_PastReadingsGameInstance.LocationMC` (`self.K2_GetActorLocation` _returnvalue) _asbp_past_readings_game_instance)
      (set `/Game/_mycontent/bp/bp_PastReadingsGameInstance.RotationMC` (`self.K2_GetActorRotation` _returnvalue) _asbp_past_readings_game_instance)
      (bind _returnvalue_2 (`GameplayStatics.GetCurrentLevelName` true))
      (`KismetSystemLibrary.PrintString` _returnvalue_2)
      (set `/Game/_mycontent/bp/bp_PastReadingsGameInstance.RoomMC` (`KismetStringLibrary.EqualEqual_StrStr` _returnvalue_2 "lvl_garden") _asbp_past_readings_game_instance)
      (`GameplayStatics.PlaySound2D` "/Game/_mycontent/sound/sfx/sfx_found-card.sfx_found-card" 0.4 1.0 0.0 null null)
      (`KismetSystemLibrary.Delay` 1.0)
      (bind _asbp_past_readings_game_instance_2 (cast `/Game/_mycontent/bp/bp_PastReadingsGameInstance` (`GameplayStatics.GetGameInstance`)))
      (set `/Game/_mycontent/bp/bp_PastReadingsGameInstance.CardFoundINT` 4 _asbp_past_readings_game_instance_2)
      (bind _returnvalue_3 (`|CreateWidget` "/Game/Movies/VideoPlayer.VideoPlayer_C" null "/Game/Movies/CineMaterial_Inicio.CineMaterial_Inicio"))
      (`UserWidget.AddToViewport` _returnvalue_3 0)
      (`MediaPlayer.OpenSource` (`self.Target`) "/Game/Movies/Cine_Final.Cine_Final")
      (`KismetSystemLibrary.Delay` 7.8)
      (`GameplayStatics.OpenLevelBySoftObjectPtr` "/Game/_CardGameMyContent/lvl_CardsTabletop.lvl_CardsTabletop"))))

(fn `CheckSpeaking`
  (returns (bSpeak :type Boolean))
  (return false))

(fn `UserConstructionScript`)