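; Game instance that holds card and game progress, handles the single save slot and opens the menu level.
; Init splits the card array in half between main room and garden.
; Saving copies progress, card arrays, player transform and a garden/main-room flag into the save object.
; Loading restores from that in-memory object, which Continue reads from disk, then requests the flagged level and immediately sets the current pawn's transform.
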(event `self.ReceiveInit`
  (bind _arraycards (`self.arrayCards`))
  (for (_array_element _array_index) _arraycards
    (if (< _array_index (/ (`KismetArrayLibrary.Array_Length` _arraycards) 2))
      (`KismetArrayLibrary.Array_Add` (`self.arrayCardsMainroom`) _array_element)
      (else
        (`KismetArrayLibrary.Array_Add` (`self.arrayCardsGarden`) _array_element)))))

(event `SaveGame`
  (bind _returnvalue (`GameplayStatics.GetPlayerPawn` 0))
  (bind _bpsavegame (`self.bpSaveGame`))
  ;[0.502 1 0.8706] GUARDAR
  (bind _returnvalue_2 (`GameplayStatics.DoesSaveGameExist` "save1" :!label _label))
  (if _returnvalue_2
    (bind _asbp_past_readings_game_instance (cast `/Game/_mycontent/bp/bp_PastReadingsGameInstance` (`GameplayStatics.GetGameInstance`)))
    (if (== (`GameplayStatics.GetObjectClass` _returnvalue) "/Game/ThirdPerson/Blueprints/BP_ThirdPersonCharacter.BP_ThirdPersonCharacter_C")
      (set `/Game/_mycontent/bp/bp_PastReadingsGameInstance.LocationMC` (`Actor.K2_GetActorLocation` _returnvalue) _asbp_past_readings_game_instance)
      (set `/Game/_mycontent/bp/bp_PastReadingsGameInstance.RotationMC` (`Actor.K2_GetActorRotation` _returnvalue) _asbp_past_readings_game_instance)
      (bind _returnvalue_3 (`GameplayStatics.GetCurrentLevelName` true))
      (set `/Game/_mycontent/bp/bp_PastReadingsGameInstance.RoomMC` (`KismetStringLibrary.EqualEqual_StrStr` _returnvalue_3 "lvl_garden") _asbp_past_readings_game_instance))
    (set `/Game/_mycontent/bp/bp_savegame.LocationMC` (`self.LocationMC`) _bpsavegame)
    (set `/Game/_mycontent/bp/bp_savegame.RoomMC` (`self.RoomMC`) _bpsavegame)
    (set `/Game/_mycontent/bp/bp_savegame.RotationMC` (`self.RotationMC`) _bpsavegame)
    (set `/Game/_mycontent/bp/bp_savegame.CardsGot` (`self.CardsGot`) _bpsavegame)
    (set `/Game/_mycontent/bp/bp_savegame.LostGames` (`self.LostGames`) _bpsavegame)
    (set `/Game/_mycontent/bp/bp_savegame.WonGames` (`self.WonGames`) _bpsavegame)
    (set `/Game/_mycontent/bp/bp_savegame.arrayCardsGarden` (`self.arrayCardsGarden`) _bpsavegame)
    (set `/Game/_mycontent/bp/bp_savegame.arrayCardsMainroom` (`self.arrayCardsMainroom`) _bpsavegame)
    (`GameplayStatics.SaveGameToSlot` _bpsavegame "save1")
    (`KismetSystemLibrary.PrintString` "Saved")
    (else
      (bind _returnvalue_4 (`GameplayStatics.CreateSaveGameObject` "/Game/_mycontent/bp/bp_savegame.bp_savegame_C"))
      (set `self.bpSaveGame` _returnvalue_4))))

(event `/Game/ThirdPerson/Blueprints/bpi_player.CharacterSave`
  ;[0.502 1 0.8706] GUARDAR
  (goto _label))

(event `LoadGame`
  (bind _returnvalue (`GameplayStatics.GetPlayerPawn` 0))
  (bind _bpsavegame (`self.bpSaveGame`))
  ;[0.502 1 0.8706] CARGAR
  (bind _returnvalue_2 (`GameplayStatics.DoesSaveGameExist` "save1" :!label _label_2))
  (if _returnvalue_2
    (set `self.LocationMC` (`/Game/_mycontent/bp/bp_savegame.LocationMC` _bpsavegame))
    (set `self.RoomMC` (`/Game/_mycontent/bp/bp_savegame.RoomMC` _bpsavegame))
    (set `self.RotationMC` (`/Game/_mycontent/bp/bp_savegame.RotationMC` _bpsavegame))
    (set `self.CardsGot` (`/Game/_mycontent/bp/bp_savegame.CardsGot` _bpsavegame))
    (set `self.LostGames` (`/Game/_mycontent/bp/bp_savegame.LostGames` _bpsavegame))
    (set `self.WonGames` (`/Game/_mycontent/bp/bp_savegame.WonGames` _bpsavegame))
    (set `self.arrayCardsGarden` (`/Game/_mycontent/bp/bp_savegame.arrayCardsGarden` _bpsavegame))
    (set `self.arrayCardsMainroom` (`/Game/_mycontent/bp/bp_savegame.arrayCardsMainroom` _bpsavegame))
    (if (`self.RoomMC`)
      (`GameplayStatics.OpenLevelBySoftObjectPtr` "/Game/_mycontent/levels/lvl_garden.lvl_garden")
      (else
        (`GameplayStatics.OpenLevelBySoftObjectPtr` "/Game/_mycontent/levels/lvl_mainroom.lvl_mainroom")))
    (`Actor.K2_SetActorLocation` _returnvalue (`self.LocationMC`) false false)
    (`Actor.K2_SetActorRotation` _returnvalue (`self.RotationMC`) false)
    (`KismetSystemLibrary.PrintString` "Loaded")))

(event `/Game/ThirdPerson/Blueprints/bpi_player.CharacterLoad`
  ;[0.502 1 0.8706] CARGAR
  (goto _label_2))

(event `/Game/ThirdPerson/Blueprints/bpi_player.CharacterContinue`
  ;[0.502 1 0.8706] guardado inicio
  (bind _returnvalue (`GameplayStatics.LoadGameFromSlot` "save1" :!label _label_3))
  (bind _asbp_savegame (cast `/Game/_mycontent/bp/bp_savegame` _returnvalue))
  (set `self.bpSaveGame` _asbp_savegame))

(event `/Game/ThirdPerson/Blueprints/bpi_player.CharacterSaveInitial`
  ;[0.502 1 0.8706] guardado inicio
  (bind _returnvalue (`GameplayStatics.DoesSaveGameExist` "save1"))
  (if _returnvalue
    (goto _label_3)
    (else
      ;;[0.502 1 0.8706] generar guardado
      (bind _returnvalue_2 (`GameplayStatics.CreateSaveGameObject` "/Game/_mycontent/bp/bp_savegame.bp_savegame_C"))
      (bind _output_get (set `self.bpSaveGame` _returnvalue_2))
      (`GameplayStatics.SaveGameToSlot` _output_get "save1")
      (`KismetSystemLibrary.PrintString` "INIT")
      (`self.SaveGame`)
      (`KismetSystemLibrary.PrintString` "AFTER"))))

(event `/Game/ThirdPerson/Blueprints/bpi_player.CharacterMenu`
  (`GameplayStatics.OpenLevelBySoftObjectPtr` "/Game/_mycontent/levels/lvl_menu.lvl_menu"))

(fn `CheckSpeaking`
  (returns (bSpeak :type Boolean))
  (return false))