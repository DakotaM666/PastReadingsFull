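; Mirror ball Blueprint that spins its mesh and point light while changing the light to random colors.
; Tick rotates both components in yaw, scaled by delta time and a Rotation variable.
; A Delay on Tick throttles ChangeColor to roughly every 0.8 seconds, converting a random unit vector into the light color.
; BeginPlay sets a one-second timer without a function name.
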(event `self.ReceiveBeginPlay`
  ;[1 0.2147 0.5] beginplay
  (`KismetSystemLibrary.K2_SetTimer` null "" 1.0))

(event `self.ReceiveTick`
  (params (DeltaSeconds :type "Float (single-precision)"))
  (bind _returnvalue (* DeltaSeconds (`self.Rotation`)))
  ;[1 0.4271 0.6965] rotación luces y bola
  (`SceneComponent.K2_AddLocalRotation` (`self.PointLight`) (`KismetMathLibrary.MakeRotator` 0.0 0.0 _returnvalue) false false)
  (`SceneComponent.K2_AddLocalRotation` (`self.StaticMesh`) (`KismetMathLibrary.MakeRotator` 0.0 0.0 _returnvalue) false false)
  (`KismetSystemLibrary.Delay` 0.8)
  (`self.change color`))

(event `change color`
  ;[1 0.4597 0.7659] cambio color
  (`LightComponent.SetLightColor` (`self.PointLight`) (`KismetMathLibrary.Conv_VectorToLinearColor` (`KismetMathLibrary.RandomUnitVector`)) true))

(fn `UserConstructionScript`)