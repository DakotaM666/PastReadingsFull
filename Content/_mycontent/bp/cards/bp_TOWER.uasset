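; Collectible Tower card that the player finds by interacting with it, ending the current level.
; Interact spawns a Niagara effect at the card and plays a found-card sound.
; After a short delay it records this card as CardFound in the PastReadings game instance, then opens the menu level.
; CheckSpeaking always returns false.
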(event `/Game/ThirdPerson/Blueprints/bpi_player.Interact`
  (if true
    (`NiagaraFunctionLibrary.SpawnSystemAtLocation` "/Game/_mycontent/effects/cardFound/ns_cardtest.ns_cardtest" (.location (`self.GetTransform`)) (.rotation (`self.GetTransform`)) (2.0 2.0 2.0))
    (`GameplayStatics.PlaySound2D` "/Game/_mycontent/sound/sfx/sfx_found-card.sfx_found-card" 1.0 1.0 0.0 null null)
    (`KismetSystemLibrary.Delay` 3.0)
    (bind _asbp_past_readings_game_instance (cast `/Game/_mycontent/bp/bp_PastReadingsGameInstance` (`GameplayStatics.GetGameInstance`)))
    (set `/Game/_mycontent/bp/bp_PastReadingsGameInstance.CardFound` "bp_TOWER_C" _asbp_past_readings_game_instance)
    (`GameplayStatics.OpenLevelBySoftObjectPtr` "/Game/_mycontent/levels/lvl_menu.lvl_menu")))

(fn `CheckSpeaking`
  (returns (bSpeak :type Boolean))
  (return false))

(fn `UserConstructionScript`)