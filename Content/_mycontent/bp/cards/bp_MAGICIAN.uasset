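; Interactable Magician tarot card pickup that sends the player to the card tabletop level when found.
; Interact only proceeds if the game instance holds card 0 but not card 1.
; It saves the player's transform and whether the level is the garden, plays Niagara and sound effects, and records the found card.
; A video widget then plays a cinematic, with a fixed delay timing the level switch.
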(event `/Game/ThirdPerson/Blueprints/bpi_player.Interact`
  (bind _returnvalue (`GameplayStatics.GetPlayerPawn` 0))
  (bind _asbp_past_readings_game_instance (cast `/Game/_mycontent/bp/bp_PastReadingsGameInstance` (`GameplayStatics.GetGameInstance`)))
  (bind _cardsgot (`/Game/_mycontent/bp/bp_PastReadingsGameInstance.CardsGot` _asbp_past_readings_game_instance))
  (if (`KismetArrayLibrary.Array_Contains` _cardsgot)
    (if (not (`KismetArrayLibrary.Array_Contains` _cardsgot 1))
      (set `/Game/_mycontent/bp/bp_PastReadingsGameInstance.LocationMC` (`self.K2_GetActorLocation` _returnvalue) _asbp_past_readings_game_instance)
      (set `/Game/_mycontent/bp/bp_PastReadingsGameInstance.RotationMC` (`self.K2_GetActorRotation` _returnvalue) _asbp_past_readings_game_instance)
      (bind _returnvalue_2 (`GameplayStatics.GetCurrentLevelName` true))
      (`KismetSystemLibrary.PrintString` _returnvalue_2)
      (set `/Game/_mycontent/bp/bp_PastReadingsGameInstance.RoomMC` (`KismetStringLibrary.EqualEqual_StrStr` _returnvalue_2 "lvl_garden") _asbp_past_readings_game_instance)
      (`NiagaraFunctionLibrary.SpawnSystemAtLocation` "/Game/_mycontent/effects/cardFound/ns_cardtest.ns_cardtest" (.location (`self.GetTransform`)) (.rotation (`self.GetTransform`)) (2.0 2.0 2.0))
      (`GameplayStatics.PlaySound2D` "/Game/_mycontent/sound/sfx/sfx_found-card.sfx_found-card" 1.0 1.0 0.0 null null)
      (`KismetSystemLibrary.Delay` 0.5)
      (bind _asbp_past_readings_game_instance_2 (cast `/Game/_mycontent/bp/bp_PastReadingsGameInstance` (`GameplayStatics.GetGameInstance`)))
      (set `/Game/_mycontent/bp/bp_PastReadingsGameInstance.CardFound` "bp_MAGICIAN_C" _asbp_past_readings_game_instance_2)
      (set `/Game/_mycontent/bp/bp_PastReadingsGameInstance.CardFoundINT` 1 _asbp_past_readings_game_instance_2)
      (bind _returnvalue_3 (`|CreateWidget` "/Game/Movies/VideoPlayer.VideoPlayer_C" null "/Game/Movies/CineMaterial_Inicio.CineMaterial_Inicio"))
      (`UserWidget.AddToViewport` _returnvalue_3 0)
      (`MediaPlayer.OpenSource` (`self.Target`) "/Game/Movies/Cine_Lamp.Cine_Lamp")
      (`KismetSystemLibrary.Delay` 11.8)
      (`GameplayStatics.OpenLevelBySoftObjectPtr` "/Game/_CardGameMyContent/lvl_CardsTabletop.lvl_CardsTabletop"))))

(fn `CheckSpeaking`
  (returns (bSpeak :type Boolean))
  (return false))

(fn `UserConstructionScript`)